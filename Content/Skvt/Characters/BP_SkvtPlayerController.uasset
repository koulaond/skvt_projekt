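; BP_SkvtPlayerController is a player controller that lets the player swap control between BP_SkvtBaseChar characters in the level.
; On BeginPlay it enables input, then adds and registers the IMC_Default Enhanced Input mapping context.
; IA_Swap gathers every BP_SkvtBaseChar and possesses the one after the current pawn in that array, wrapping back to the first.
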(event Input|EnhancedActionEvents|EnhancedInputActionIA_Swap
  (params (ActionValue :type Boolean) (ElapsedSeconds :type Float%20%28double-precision%29) (TriggeredSeconds :type Float%20%28double-precision%29) (InputAction :type Input%20Action%20Object%20Reference :default "/Game/Skvt/Characters/Input/Actions/IA_Swap.IA_Swap"))
  (bind _outactors (Actor|GetAllActorsOfClass "/Game/Skvt/Characters/BP_SkvtBaseChar.BP_SkvtBaseChar_C"))
  (Pawn|Possess (CallFunction|FindCharactertoPossess _outactors)))

(event EventBeginPlay
  (bind _self self)
  (bind _returnvalue (PlayerController|LocalPlayerSubsystems|GetEnhancedInputLocalPlayerSubsystem _self))
  (Input|EnableInput (Game|GetPlayerController 0))
  (Utilities|IsValid _returnvalue
    (:Is%20Valid
      (Input|AddMappingContext _returnvalue "/Game/ThirdPerson/Input/IMC_Default.IMC_Default" 0 "(bIgnoreAllPressedKeysUntilRelease=True,bForceImmediately=False,bNotifyUserSettings=False)")
      (Class|EnhancedInputUserSettings|RegisterInputMappingContext (Class|EnhancedInputSubsystemInterface|GetUserSettings _returnvalue) "/Game/ThirdPerson/Input/IMC_Default.IMC_Default"))))

(fn ConstructionScript)

(fn FindCharactertoPossess
  (params (CHaracter :type Array%20of%20BP%20Skvt%20Base%20Char%20Object%20References))
  (bind _asbp_skvt_base_char (Utilities|Casting|CastToBP_SkvtBaseChar (Pawn|GetControlledPawn))
    (:then
      (if (== (Utilities|Array|Length CHaracter) (+ (Utilities|Array|FindItem CHaracter _asbp_skvt_base_char) 1))
        (return (Utilities|Array|Get(acopy) CHaracter))
        (else
          (return (Utilities|Array|Get(acopy) CHaracter (+ (Utilities|Array|FindItem CHaracter _asbp_skvt_base_char) 1))))))
    (:CastFailed
      (Development|PrintString "Cast failed"))))